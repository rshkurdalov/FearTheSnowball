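; BP_AI is a slow-walking AI character that follows a destination actor and detonates when close to it.
; StartFolowing stores the target and starts an AI MoveTo; afterwards ChangeTarget waits, then restarts following the same DestinationActor.
; Tick checks whether the target is within Distance, without a validity check, then fires the detonate dispatcher and destroys the character.
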(event `self.ReceiveBeginPlay`
  (set `CharacterMovementComponent.MaxWalkSpeed` 100.0 (`self.CharacterMovement`)))

(event `OnStartFollowing`
  (bind _destinationactor (`self.DestinationActor`))
  (`/Engine/EditorBlueprintResources/StandardMacros.IsValid` _destinationactor
    (:`Is Valid`
      (`AITask_MoveTo.AIMoveTo` (`AIBlueprintHelperLibrary.GetAIController` self) (0.0 0.0 0.0) _destinationactor 5.0
        (:`then`
          (`self.ChangeTarget`))))))

(event `ChangeTarget`
  (`KismetSystemLibrary.Delay` 8.5)
  (`KismetSystemLibrary.PrintString` "Start folowing new actor")
  (`self.StartFolowing` (`self.DestinationActor`)))

(event `self.ReceiveTick`
  (params (DeltaSeconds :type "Float (single-precision)"))
  (bind _canbeblown (`self.CanBeBlown`))
  (if _canbeblown
    (`self.Detonate`)))

(fn `CanBeBlown`
  (returns (CanBeBlown :type Boolean))
  (return (< (`KismetMathLibrary.VSize` (- (`self.K2_GetActorLocation` (`self.DestinationActor`)) (`self.K2_GetActorLocation`))) (`self.Distance`))))

(fn `Detonate`
  (`KismetSystemLibrary.PrintText` "DETONATE" true true (struct :`R` 1.0 :`G` 0.072804 :`A` 1.0))
  (`self.DetonateEventDispatcher`)
  (`self.K2_DestroyActor`))

(fn `StartFolowing`
  (params (Destination :type "Actor Object Reference"))
  (set `self.DestinationActor` Destination)
  (`self.OnStartFollowing`))

(fn `UserConstructionScript`)