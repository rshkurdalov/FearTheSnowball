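; Exploding AI character that chases a random player and blows up on proximity.
; On the server, looping timers drive targeting, validation and blast checks.
; Targets are picked from players standing on the navmesh and followed with AIMoveTo; one leaving it forces reselection and restarts the 10-second retarget timer.
; A player within Distance gets launched away and upward, then the AI fires its detonate dispatcher and destroys itself.
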(event `self.ReceiveBeginPlay`
  (`/Engine/EditorBlueprintResources/ActorMacros.Switch Has Authority`
    (:`Authority`
      (set `CharacterMovementComponent.MaxWalkSpeed` 100.0 (`self.CharacterMovement`))
      (`|ExecutionSequence`
        (:`then_0`
          (`KismetSystemLibrary.K2_SetTimerDelegate` (`|CreateDelegate` :!event `TrySelectNewTarget`) 0.2 true))
        (:`then_1`
          (bind _returnvalue (`KismetSystemLibrary.K2_SetTimerDelegate` (`|CreateDelegate` :!event `SelectNewTarget`) 10.0 true))
          (set `self.SelectNewTargetTimerHandler` _returnvalue))
        (:`then_2`
          (`KismetSystemLibrary.K2_SetTimerDelegate` (`|CreateDelegate` :!event `TryToBlowUp`) 0.05 true))
        (:`then_3`
          (`KismetSystemLibrary.K2_SetTimerDelegate` (`|CreateDelegate` :!event `ValidateTheTarget`) 0.05 true))))))

(event `ValidateTheTarget`
  (bind _targetcharacter (`self.TargetCharacter`))
  (if (`KismetSystemLibrary.IsValid` _targetcharacter)
    (if (not (`.ReturnValue` (`NavigationSystemV1.K2_ProjectPointToNavigation` (`self.K2_GetActorLocation` _targetcharacter))))
      (`self.SelectNewTarget`)
      (`KismetSystemLibrary.K2_ClearAndInvalidateTimerHandle` (`self.SelectNewTargetTimerHandler`))
      (bind _returnvalue (`KismetSystemLibrary.K2_SetTimerDelegate` (`|CreateDelegate` :!event `SelectNewTarget`) 10.0 true))
      (set `self.SelectNewTargetTimerHandler` _returnvalue))))

(event `TrySelectNewTarget`
  (if (not (`self.NewTargetSelected`))
    (bind (_istargetexist _playercharacter) (`self.Get Random Target`))
    (if _istargetexist
      (bind _output_get (set `self.TargetCharacter` _playercharacter))
      (`AITask_MoveTo.AIMoveTo` (`AIBlueprintHelperLibrary.GetAIController` self) (0.0 0.0 0.0) _output_get 5.0
        (:`then`
          (set `self.NewTargetSelected` true)))
      (else
        (`KismetSystemLibrary.PrintString` "Target Player cannot be found " true true (struct :`G` 0.2155 :`B` 1.0 :`A` 1.0))))))

(event `SelectNewTarget`
  (set `self.NewTargetSelected` false))

(event `TryToBlowUp`
  (bind (_canbeblown _explodedone) (`self.CanBeBlown`))
  (if _canbeblown
    (bind _asplayer_character (cast `PlayerCharacter` _explodedone)
      (:`then`
        (`self.PunchTouchedChar` _asplayer_character)
        (`self.Detonate`))
      (:`CastFailed`
        (`KismetSystemLibrary.PrintString` "Player Controller Cast Failed")))))

(fn `CanBeBlown`
  (returns (CanBeBlown :type Boolean) (ExplodedOne :type "Actor Object Reference"))
  (bind _returnvalue (`GameModeBase.GetNumPlayers` (`GameplayStatics.GetGameMode`)))
  (for _index (range _returnvalue)
    (bind _returnvalue_2 (`GameplayStatics.GetPlayerCharacter` _index))
    (bind _returnvalue_3 (< (`KismetMathLibrary.VSize` (- (`self.K2_GetActorLocation` _returnvalue_2) (`self.K2_GetActorLocation`))) (`self.Distance`)))
    (if _returnvalue_3
      (return _returnvalue_3 _returnvalue_2)))
  (return false null))

(fn `Detonate`
  (`KismetSystemLibrary.PrintText` "DETONATE" true true (struct :`R` 1.0 :`G` 0.072804 :`A` 1.0))
  (`self.DetonateEventDispatcher`)
  (`self.K2_DestroyActor`))

(fn `Get Random Target`
  (returns (IsTargetExist :type Boolean) (PlayerCharacter :type "Character Object Reference"))
  (`KismetArrayLibrary.Array_Clear` (`self.PlayerCharacters`))
  (bind _returnvalue (`GameModeBase.GetNumPlayers` (`GameplayStatics.GetGameMode`)))
  (for _index (range _returnvalue)
    (bind _returnvalue_2 (`GameplayStatics.GetPlayerCharacter` _index))
    (if (`.ReturnValue` (`NavigationSystemV1.K2_ProjectPointToNavigation` (`self.K2_GetActorLocation` _returnvalue_2) null null (0.0 0.0 0.0)))
      (`KismetArrayLibrary.Array_Add` (`self.PlayerCharacters`) _returnvalue_2)))
  (if (> (`KismetArrayLibrary.Array_Length` (`self.PlayerCharacters`)) 0)
    (`KismetArrayLibrary.Array_Shuffle` (`self.PlayerCharacters`))
    (return true (`KismetArrayLibrary.Array_Random` (`self.PlayerCharacters`)))
    (else
      (return false null))))

(fn `PunchTouchedChar`
  (params (InputPin :type "PlayerCharacter Object Reference"))
  (bind (_returnvalue_x _returnvalue_y) (`KismetMathLibrary.BreakVector` (- (`self.K2_GetActorLocation` InputPin) (`self.K2_GetActorLocation`))))
  (`self.LaunchCharacter` InputPin (+ (* (`KismetMathLibrary.MakeVector` _returnvalue_x _returnvalue_y) 10.0) (`KismetMathLibrary.MakeVector` 0.0 0.0 200.0)) false false))

(fn `UserConstructionScript`)