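; Spawner actor that keeps a capped population of BP_AI actors alive at its SpawnPoint.
; From BeginPlay, OnSpawnFolower re-calls itself after a fixed delay, calling SpawnAI whenever SpawnedCount is below MaxSpawnCount.
; SpawnAI increments the count and binds to each AI's detonate dispatcher, while OnDetonateFunc decrements the count to free a slot.
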(event `self.ReceiveBeginPlay`
  (`self.OnSpawnFolower`))

(event `OnSpawnFolower`
  (`KismetSystemLibrary.PrintString` "Spawn")
  (if (not (>= (`self.SpawnedCount`) (`self.MaxSpawnCount`)))
    (`self.SpawnAI`))
  (`KismetSystemLibrary.Delay` 5.0)
  (`self.OnSpawnFolower`))

(fn `OnDetonateFunc`
  (set `self.SpawnedCount` (- (`self.SpawnedCount`) 1)))

(fn `SpawnAI`
  (bind _returnvalue (`|SpawnActorFromClass` "/Game/BP/BP_AI.BP_AI_C" (`SceneComponent.K2_GetComponentToWorld` (`self.SpawnPoint`)) "Undefined" "OverrideRootScale" null null))
  (add `/Game/BP/BP_AI.DetonateEventDispatcher` _returnvalue (`|CreateDelegate` :!event `OnDetonateFunc`))
  (set `self.SpawnedCount` (+ (`self.SpawnedCount`) 1)))

(fn `UserConstructionScript`)