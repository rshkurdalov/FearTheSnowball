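; BP_CapturePoint is a capture point actor that displays its state through a decal.
; On BeginPlay it creates a dynamic material instance for the decal and prints whether it has authority as a debug string.
; The OnPointRadiusChange event drives the material's grow direction, fill radius and inner color parameters, leaving the visual fill to the material.
; The Blueprint holds no capture logic, only this visual response.
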(event `self.ReceiveBeginPlay`
  (bind _returnvalue (`DecalComponent.CreateDynamicMaterialInstance` (`self.Decal`)))
  (set `self.DecalMaterial` _returnvalue)
  (`KismetSystemLibrary.PrintString` (`KismetStringLibrary.Conv_BoolToString` (`self.HasAuthority`))))

(event `self.OnPointRadiusChange`
  (params (ChangeDirection :type "Float (single-precision)") (NewFillRadius :type "Float (single-precision)") (PointColor :type "Color Structure"))
  (bind _decalmaterial (`self.DecalMaterial`))
  (`|ExecutionSequence`
    (:`then_0`
      (`MaterialInstanceDynamic.SetScalarParameterValue` _decalmaterial "GrowDirection" ChangeDirection))
    (:`then_1`
      (`MaterialInstanceDynamic.SetScalarParameterValue` _decalmaterial "FillRadius" NewFillRadius))
    (:`then_2`
      (`MaterialInstanceDynamic.SetVectorParameterValue` _decalmaterial "InnerColor" (`KismetMathLibrary.Conv_ColorToLinearColor` PointColor)))))

(fn `UserConstructionScript`)